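; BP_NPC is an AI-driven character that carries a health bar widget and shows an outline when the player is near.
; A movement state sets walk speed, and the sphere collider toggles an overlay material on the mesh.
; Hit and death events extend parent logic: hits halt movement and play a montage that clears attacking on blend-out, while death stops the AI brain.
; Getters expose the behavior tree and the NPC itself.
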(event OnComponentBeginOverlap(SphereCollider)
  (params (OverlappedComponent :type Primitive%20Component%20Object%20Reference) (OtherActor :type Actor%20Object%20Reference) (OtherComp :type Primitive%20Component%20Object%20Reference) (OtherBodyIndex :type Integer) (bFromSweep :type Boolean) (SweepResult :type Hit%20Result%20Structure%20%28by%20ref%29))
  (Utilities|Casting|CastToBP_Player OtherActor)
  (Rendering|Material|SetOverlayMaterial (Variables|Character|GetMesh) "/Game/Art/Materials/MO_Outline.MO_Outline" :!class /Script/Engine.MeshComponent))

(event OnComponentEndOverlap(SphereCollider)
  (params (OverlappedComponent :type Primitive%20Component%20Object%20Reference) (OtherActor :type Actor%20Object%20Reference) (OtherComp :type Primitive%20Component%20Object%20Reference) (OtherBodyIndex :type Integer))
  (Utilities|Casting|CastToBP_Player OtherActor)
  (Rendering|Material|SetOverlayMaterial (Variables|Character|GetMesh) 0 :!class /Script/Engine.MeshComponent))

(event Custom|SetMovementState
  (params (NewState :type E_AIMovement%20Enum :default "NewEnumerator0"))
  ;[0 0 0] Movement State
  (Variables|/Script/Engine.CharacterMovementComponent|SetMaxWalkSpeed (Variables|Character|GetCharacterMovement) (Utilities|Select :Index NewState :NewEnumerator0 0.0 :NewEnumerator1 1.5e+02 :NewEnumerator2 5e+02)))

(event EventBeginPlay
  ;[0 0 0] Begin play
  (bind _returnvalue (UserInterface|CreateWidget "/Game/System/Widgets/WBP_Healthbar.WBP_Healthbar_C" 0 self))
  (UserInterface|SetWidget (Variables|Default|GetHealthbar) _returnvalue))

(event EventOnHit
  ;[0 0 0] On hit
  (|CallParentFunction)
  (Components|Movement|StopMovementImmediately (Variables|Character|GetCharacterMovement))
  (Animation|Montage|PlayMontage (Variables|Character|GetMesh) (Variables|Default|GetHitMontage)
    (:OnBlendOut
      (Variables|Default|SetbAttacking false)
      (Default|CallOnHitEnd))))

(event EventOnDeath
  (bind _self self)
  (bind _returnvalue (AI|GetAIController _self))
  (bind _braincomponent (Variables|/Script/AIModule.AIController|GetBrainComponent _returnvalue))
  ;[0 0 0] On death
  (|CallParentFunction)
  (Utilities|IsValid _braincomponent
    (:Is%20Valid
      (AI|Logic|StopLogic _braincomponent "Dead"))))

(fn ConstructionScript
  (|CallParentFunction))

(fn GetBehaviorTree
  (return (Variables|Default|GetBehaviorTree)))

(fn GetNPC
  (return self))