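; Player character Blueprint for a cursor-aimed action game with melee and ranged combat, potions, interaction and quests.
; Enhanced Input events drive movement, parent combat actions and UI widgets, rotating the capsule toward the cursor while attacking or shooting.
; Health, ammo and quests save through the GameInstance and reload on BeginPlay; death shows a restart widget.
; Tick turns the aim sprite and hides "ToHidde"-tagged objects blocking the camera; debug keys are included.
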(event Input|EnhancedActionEvents|EnhancedInputActionIA_Move
  (params (ActionValue :type Vector%202D%20Structure) (ElapsedSeconds :type Float%20%28double-precision%29) (TriggeredSeconds :type Float%20%28double-precision%29) (InputAction :type Input%20Action%20Object%20Reference :default "/Game/System/Inputs/Actions/IA_Move.IA_Move"))
  (bind _returnvalue (Pawn|GetBaseAimRotation))
  ;[0 0 0] Movement
  (Pawn|Input|AddMovementInput (Math|Vector|GetRightVector (Math|Rotator|MakeRotator (.roll _returnvalue) 0.0 (.yaw _returnvalue))) (.x ActionValue) false) ; Left and right
  (Pawn|Input|AddMovementInput (Math|Vector|GetForwardVector (Math|Rotator|MakeRotator 0.0 0.0 (.yaw _returnvalue))) (.y ActionValue) false) ; Up and down
)

(event Input|EnhancedActionEvents|EnhancedInputActionIA_Toggle-Melee
  (params (ActionValue :type Boolean) (ElapsedSeconds :type Float%20%28double-precision%29) (TriggeredSeconds :type Float%20%28double-precision%29) (InputAction :type Input%20Action%20Object%20Reference :default "/Game/System/Inputs/Actions/IA_Toggle-Melee.IA_Toggle-Melee"))
  ;[0 0 0] Weapon toggle
  (:Started
    (CallFunction|AddWeapon "NewEnumerator0" "NewEnumerator1")
    (Audio|SpawnSound2D "/Game/Art/Sounds/Meta/MS_GetItem.MS_GetItem" 1.0 1.0 0.0 0)))

(event Input|EnhancedActionEvents|EnhancedInputActionIA_Journal
  (params (ActionValue :type Boolean) (ElapsedSeconds :type Float%20%28double-precision%29) (TriggeredSeconds :type Float%20%28double-precision%29) (InputAction :type Input%20Action%20Object%20Reference :default "/Game/System/Inputs/Actions/IA_Journal.IA_Journal"))
  ;[0 0 0] Journal
  (:Started
    (bind _returnvalue (UserInterface|CreateWidget "/Game/System/Widgets/WBP_Journal.WBP_Journal_C"))
    (Default|AddQuesttoList _returnvalue (Variables|Default|GetQuests))
    (UserInterface|Viewport|AddtoViewport _returnvalue 0)
    (Input|DisableInput (Game|GetPlayerController 0))))

(event Input|EnhancedActionEvents|EnhancedInputActionIA_Menu-Game
  (params (ActionValue :type Boolean) (ElapsedSeconds :type Float%20%28double-precision%29) (TriggeredSeconds :type Float%20%28double-precision%29) (InputAction :type Input%20Action%20Object%20Reference :default "/Game/System/Inputs/Actions/IA_Menu-Game.IA_Menu-Game"))
  ;[0 0 0] Game menu
  (:Started
    (bind _returnvalue (UserInterface|CreateWidget "/Game/System/Widgets/WBP_MenuGame.WBP_MenuGame_C" 0 self))
    (UserInterface|Viewport|AddtoViewport _returnvalue 0)
    (Input|DisableInput (Game|GetPlayerController 0))))

(event Input|EnhancedActionEvents|EnhancedInputActionIA_Interact
  (params (ActionValue :type Boolean) (ElapsedSeconds :type Float%20%28double-precision%29) (TriggeredSeconds :type Float%20%28double-precision%29) (InputAction :type Input%20Action%20Object%20Reference :default "/Game/System/Inputs/Actions/IA_Interact.IA_Interact"))
  (bind _returnvalue (Transformation|GetActorLocation))
  ;[0 0 0] Interact
  (:Started
    (bind _outhit (Collision|SphereTraceForObjects _returnvalue _returnvalue 5e+01 (Utilities|Array|MakeArray "ObjectTypeQuery3" "ObjectTypeQuery2") false (Utilities|Array|MakeArray self) "None" true "(R=1.000000,G=0.000000,B=0.000000,A=1.000000)" "(R=0.000000,G=1.000000,B=0.000000,A=1.000000)" 1.0))
    (Class|BPIInteractive|Interact(Message) (.HitActor (Collision|BreakHitResult _outhit)) self)))

(event Input|EnhancedActionEvents|EnhancedInputActionIA_DrinkPotion
  (params (ActionValue :type Boolean) (ElapsedSeconds :type Float%20%28double-precision%29) (TriggeredSeconds :type Float%20%28double-precision%29) (InputAction :type Input%20Action%20Object%20Reference :default "/Game/System/Inputs/Actions/IA_DrinkPotion.IA_DrinkPotion"))
  ;[0 0 0] Drink potion
  (:Started
    (if (> (Variables|Default|GetHealthPotions) 0)
      (Variables|Default|SetCurrentHealth (Math|Float|Clamp(Float) (+ (Variables|Default|GetCurrentHealth) 5e+01) 0.0 (Variables|Default|GetMaxHealth)))
      (Math|Integer|DecrementInt (Variables|Default|GetHealthPotions))
      (else
        (Development|PrintString "No potion" true true "(R=1.000000,G=0.000000,B=0.000000,A=1.000000)")))))

(event Input|EnhancedActionEvents|EnhancedInputActionIA_Toggle-Ranged
  (params (ActionValue :type Boolean) (ElapsedSeconds :type Float%20%28double-precision%29) (TriggeredSeconds :type Float%20%28double-precision%29) (InputAction :type Input%20Action%20Object%20Reference :default "/Game/System/Inputs/Actions/IA_Toggle-Ranged.IA_Toggle-Ranged"))
  ;[0 0 0] Weapon toggle
  (:Started
    (CallFunction|AddWeapon "NewEnumerator1" "NewEnumerator2")
    (Audio|SpawnSound2D "/Game/Art/Sounds/Meta/MS_GetItem.MS_GetItem" 1.0 1.0 0.0 0)))

(event Input|EnhancedActionEvents|EnhancedInputActionIA_Attack-Light
  (params (ActionValue :type Boolean) (ElapsedSeconds :type Float%20%28double-precision%29) (TriggeredSeconds :type Float%20%28double-precision%29) (InputAction :type Input%20Action%20Object%20Reference :default "/Game/System/Inputs/Actions/IA_Attack-Light.IA_Attack-Light"))
  ;[0 0 0] Melee actions
  (:Triggered
    (if (Variables|Default|GetbAttacking)
      (CallFunction|RotateTowardsCursor (Variables|Default|GetCapsuleComponent) "0, 0, 0")))
  (:Started
    (if (not (Variables|Default|GetbAttacking))
      (Utilities|FlowControl|FlipFlop
        (:A
          (CallFunction|LightAttack "Attack_1" 1.3 15.0))
        (:B
          (CallFunction|LightAttack "Attack_2" 1.3 15.0))))))

(event Input|EnhancedActionEvents|EnhancedInputActionIA_Attack-Heavy
  (params (ActionValue :type Boolean) (ElapsedSeconds :type Float%20%28double-precision%29) (TriggeredSeconds :type Float%20%28double-precision%29) (InputAction :type Input%20Action%20Object%20Reference :default "/Game/System/Inputs/Actions/IA_Attack-Heavy.IA_Attack-Heavy"))
  ;[0 0 0] Melee actions
  (:Triggered
    (if (Variables|Default|GetbAttacking)
      (CallFunction|RotateTowardsCursor (Variables|Default|GetCapsuleComponent) "0, 0, 0")))
  (:Started
    (if (not (Variables|Default|GetbAttacking)) ; Branch to avoid player triggering (same for light attacks)
      (CallFunction|HeavyAttack 1.2 3e+01))))

(event Input|EnhancedActionEvents|EnhancedInputActionIA_Dash
  (params (ActionValue :type Boolean) (ElapsedSeconds :type Float%20%28double-precision%29) (TriggeredSeconds :type Float%20%28double-precision%29) (InputAction :type Input%20Action%20Object%20Reference :default "/Game/System/Inputs/Actions/IA_Dash.IA_Dash"))
  ;[0 0 0] Movement actions
  (:Started
    (CallFunction|Dash)))

(event Input|EnhancedActionEvents|EnhancedInputActionIA_Toggle-Walk
  (params (ActionValue :type Boolean) (ElapsedSeconds :type Float%20%28double-precision%29) (TriggeredSeconds :type Float%20%28double-precision%29) (InputAction :type Input%20Action%20Object%20Reference :default "/Game/System/Inputs/Actions/IA_Toggle-Walk.IA_Toggle-Walk"))
  ;[0 0 0] Movement actions
  (:Started
    (CallFunction|Walk)))

(event Input|EnhancedActionEvents|EnhancedInputActionIA_Defend
  (params (ActionValue :type Boolean) (ElapsedSeconds :type Float%20%28double-precision%29) (TriggeredSeconds :type Float%20%28double-precision%29) (InputAction :type Input%20Action%20Object%20Reference :default "/Game/System/Inputs/Actions/IA_Defend.IA_Defend"))
  ;[0 0 0] Melee actions
  (:Started
    (if (not (Variables|Default|GetbDefending))
      (CallFunction|StartDefending))))

(event Input|EnhancedActionEvents|EnhancedInputActionIA_Shoot
  (params (ActionValue :type Boolean) (ElapsedSeconds :type Float%20%28double-precision%29) (TriggeredSeconds :type Float%20%28double-precision%29) (InputAction :type Input%20Action%20Object%20Reference :default "/Game/System/Inputs/Actions/IA_Shoot.IA_Shoot"))
  ;[0 0 0] Ranged actions
  (:Triggered
    (if (Variables|Default|GetbShooting)
      (CallFunction|RotateTowardsCursor (Variables|Default|GetCapsuleComponent) "0, 0, 0")))
  (:Started
    (CallFunction|StartShooting 1.7 1e+01))
  (:Completed
    (CallFunction|StopShooting)))

(event Input|EnhancedActionEvents|EnhancedInputActionIA_Reload
  (params (ActionValue :type Boolean) (ElapsedSeconds :type Float%20%28double-precision%29) (TriggeredSeconds :type Float%20%28double-precision%29) (InputAction :type Input%20Action%20Object%20Reference :default "/Game/System/Inputs/Actions/IA_Reload.IA_Reload"))
  ;[0 0 0] Ranged actions
  (:Started
    (CallFunction|Reload 1.0)))

(event EventOnDeath
  ;[0 0 0] On death
  (|CallParentFunction)
  (Widget|RemovefromParent (stale EventBeginPlay _returnvalue_3))
  (Utilities|FlowControl|Delay 2.0)
  (bind _returnvalue (UserInterface|CreateWidget "/Game/System/Widgets/WBP_RestartGame.WBP_RestartGame_C"))
  (UserInterface|Viewport|AddtoViewport _returnvalue 0)
  (Input|DisableInput (Game|GetPlayerController 0)))

(event EventBeginPlay
  (bind _returnvalue (Game|GetPlayerController 0))
  (bind _returnvalue_2 (PlayerController|LocalPlayerSubsystems|GetEnhancedInputLocalPlayerSubsystem _returnvalue))
  ;[0 0 0] Begin play
  (Utilities|IsValid _returnvalue_2
    (:Is%20Valid
      (Input|AddMappingContext _returnvalue_2 "/Game/System/Inputs/IMC_Default.IMC_Default" 0 "(bIgnoreAllPressedKeysUntilRelease=True,bForceImmediately=False,bNotifyUserSettings=False)")
      (bind _returnvalue_3 (UserInterface|CreateWidget "/Game/System/Widgets/WBP_PlayerUI.WBP_PlayerUI_C" 0 self))
      (UserInterface|Viewport|AddtoViewport _returnvalue_3 0)
      (CallFunction|UsePlayerSave true)
      (Variables|/Script/Engine.PlayerController|SetbShowMouseCursor _returnvalue true)
      (Input|SetInputModeGameandUI _returnvalue _returnvalue_3 "DoNotLock" false false))))

(event EventTick
  (params (DeltaSeconds :type Float%20%28single-precision%29))
  ;[0 0 0] Hide traced objects
  (CallFunction|HideTracedObject)
  (CallFunction|RotateTowardsCursor (Variables|Default|GetAimSprite) "0.000000,90.000000,-90.000000"))

(event Input|KeyboardEvents|DebugKeyG
  (params (Key :type Key%20Structure :default "None") (ActionValue :type Input%20Action%20Value%20Structure))
  ;[0.01555 0 0.07812] DEBUG SECTION
  (:Pressed
    (for _array_element (Variables|Default|GetQuests)
      (Development|PrintString (Utilities|GetDisplayName _array_element))
      (Development|PrintString (Utilities|String|ToString(Integer) (Variables|/Game/System/Quests/PDA_Quest.PDA_Quest_C|GetStageIndex _array_element))))))

(event Input|KeyboardEvents|DebugKeyV
  (params (Key :type Key%20Structure :default "None") (ActionValue :type Input%20Action%20Value%20Structure))
  ;[0.01555 0 0.07812] DEBUG SECTION
  (:Pressed
    (for _array_element (Utilities|Array|MakeArray "/Game/System/Quests/_Debug/DA_Quest_AdanToEve.DA_Quest_AdanToEve" "/Game/System/Quests/_Debug/DA_Quest_CainToAbel.DA_Quest_CainToAbel" "/Game/System/Quests/Prologue/DA_Qst_Prologue.DA_Qst_Prologue")
      (Default|ResetQuest _array_element)
      (Development|PrintString "Quest reseted" true true "(R=1.000000,G=1.000000,B=1.000000,A=1.000000)" 1.0))
    (Utilities|Array|Clear (Variables|Default|GetQuests))))

(event Input|KeyboardEvents|DebugKeyF
  (params (Key :type Key%20Structure :default "None") (ActionValue :type Input%20Action%20Value%20Structure))
  ;[0.01555 0 0.07812] DEBUG SECTION
  (:Pressed
    (Character|Jump))
  (:Released
    (Character|StopJumping)))

(event Input|KeyboardEvents|DebugKeyX
  (params (Key :type Key%20Structure :default "None") (ActionValue :type Input%20Action%20Value%20Structure))
  ;[0.01555 0 0.07812] DEBUG SECTION
  (:Pressed
    (Audio|SpawnSoundatLocation "/Game/Art/Sounds/Meta/MS_AttackSword.MS_AttackSword" "0, 0, 0" "0, 0, 0" 1.0 1.0 0.0 0 0)))

(fn ConstructionScript)

(fn GetPlayerData
  (return (Utilities|Struct|MakeS_PlayerSave (Transformation|GetActorTransform) (Variables|Default|GetCurrentHealth) (+ (Variables|Default|GetCharAmmo) (Variables|Default|GetWeaponAmmo)) (Variables|Default|GetQuests))))

(fn UsePlayerSave
  (params (SkipTransform :type Boolean))
  (bind _savedgame (Class|BPISaveGame|GetSavedGame(Message) (Game|GetGameInstance)))
  (Utilities|IsValid _savedgame
    (:Is%20Valid
      (Utilities|FlowControl|Sequence
        (:then_0
          (if (and (not SkipTransform) (not (== (.transform (Variables|/Game/System/Game/BP_SaveGame.BP_SaveGame_C|GetPlayerSave _savedgame)) (Math|Transform|MakeTransform "0, 0, 0"))))
            (Transformation|SetActorTransform (.transform (Variables|/Game/System/Game/BP_SaveGame.BP_SaveGame_C|GetPlayerSave _savedgame)))))
        (:then_1
          (if (not (Utilities|Array|IsEmpty (.quests (Variables|/Game/System/Game/BP_SaveGame.BP_SaveGame_C|GetPlayerSave _savedgame))))
            (Variables|Default|SetQuests (.quests (Variables|/Game/System/Game/BP_SaveGame.BP_SaveGame_C|GetPlayerSave _savedgame)))))
        (:then_2
          (if (!= (.health (Variables|/Game/System/Game/BP_SaveGame.BP_SaveGame_C|GetPlayerSave _savedgame)) 0.0)
            (Variables|Default|SetCurrentHealth (.health (Variables|/Game/System/Game/BP_SaveGame.BP_SaveGame_C|GetPlayerSave _savedgame)))))
        (:then_3
          (if (!= (.ammo (Variables|/Game/System/Game/BP_SaveGame.BP_SaveGame_C|GetPlayerSave _savedgame)) 0)
            (Variables|Default|SetCharAmmo (.ammo (Variables|/Game/System/Game/BP_SaveGame.BP_SaveGame_C|GetPlayerSave _savedgame)))))))))

(fn RotateTowardsCursor
  (params (ComponentToRotate :type Scene%20Component%20Object%20Reference) (RotationOffset :type Rotator))
  (bind (_roll _pitch _yaw) (Math|Rotator|BreakRotator RotationOffset))
  (Transformation|SetWorldRotation ComponentToRotate (Math|Rotator|MakeRotator _roll _pitch (+ _yaw (.yaw (Math|Interpolation|RInterpTo (Transformation|GetActorRotation) (Math|Rotator|FindLookatRotation (Transformation|GetActorLocation) (.Location (Collision|BreakHitResult (.HitResult (Game|Player|GetHitResultUnderCursorbyChannel (Game|GetPlayerController 0) "TraceTypeQuery1" true))))) (Utilities|Time|GetWorldDeltaSeconds) 3.6e+02)))) false false))

(fn HideTracedObject
  (bind _outhit (Collision|LineTraceForObjects (Transformation|GetWorldLocation (Variables|Camera|GetCamera)) (Transformation|GetSocketLocation (Variables|Character|GetMesh) "head") (Utilities|Array|MakeArray "ObjectTypeQuery1") false 0 "None"))
  (if (== (Variables|Default|GetLastHiddenActor) (.HitActor (Collision|BreakHitResult _outhit))) ; Check if is the same actor
    _
    (else
      (bind _lasthiddenactor (Variables|Default|GetLastHiddenActor)
        (:then
          (Rendering|SetActorHiddenInGame _lasthiddenactor false) ; Unhide the last hidden actor
        )
        (:else
          _))))
  (Utilities|IsValid (.HitActor (Collision|BreakHitResult _outhit))
    (:Is%20Valid
      (bind _output_get (Variables|Default|SetLastHiddenActor (.HitActor (Collision|BreakHitResult _outhit)))) ; Save as new hidden actor
      (Rendering|SetActorHiddenInGame _output_get (Actor|ActorHasTag _output_get "ToHidde")) ; Hidde if has tag "ToHidde"
      (Development|PrintString (Utilities|GetDisplayName _output_get) true false "(R=0.000000,G=0.660000,B=1.000000,A=1.000000)" 2.0 "HiddenActor"))))

(fn AddAmmo
  (params (AmmoAmount :type Integer))
  (Variables|Default|SetCharAmmo (+ AmmoAmount (Variables|Default|GetCharAmmo))))

(fn AddPotion
  (bind _result (Math|Integer|IncrementInt (Variables|Default|GetHealthPotions))
    (:%20%20
      (Variables|Default|SetHealthPotions (Math|Integer|Clamp(Integer) _result 0 2)))))

(fn AddShield
  (params (ShieldAmount :type Float%20%28double-precision%29))
  (Variables|Default|SetCurrentShield (Math|Float|Clamp(Float) (+ ShieldAmount (Variables|Default|GetCurrentShield)) 0.0 (Variables|Default|GetMaxShield))))

(fn GetPlayer
  (return self))

(fn IsPlayer
  (return true))

(fn PlayerContainsQuest
  (params (Quest :type PDA%20Quest%20Object%20Reference))
  (bind _quests (Variables|Default|GetQuests))
  (bind _returnvalue (Utilities|Array|ContainsItem _quests Quest))
  (if _returnvalue
    (return _returnvalue (Variables|/Game/System/Quests/PDA_Quest.PDA_Quest_C|GetStageIndex (Utilities|Array|Get(acopy) _quests (Utilities|Array|FindItem _quests Quest))))
    (else
      (return false 0))))

(fn ReceiveQuest
  (params (NewQuest :type PDA%20Quest%20Object%20Reference))
  (Utilities|Array|AddUnique (Variables|Default|GetQuests) NewQuest))

(fn SavePlayerData
  (params (Async :type Boolean))
  (Class|BPISaveGame|SavePlayerGame(Message) (Game|GetGameInstance) (Utilities|Struct|MakeS_PlayerSave "0.000000,0.000000,0.000000|0.000000,0.000000,0.000000|1.000000,1.000000,1.000000" (Variables|Default|GetCurrentHealth) (+ (Variables|Default|GetCharAmmo) (Variables|Default|GetWeaponAmmo)) (Variables|Default|GetQuests)) Async))