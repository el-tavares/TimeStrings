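; Friendly NPC Cain, who gives and completes the Cain-to-Abel quest through dialogue.
; Interact reads the quest stage through ACQuest and, at stage 0 or 2, starts the matching dialogue through ACDialogue.
; Each dialogue gets a quest callback: the first gives the quest, the second marks it completed and fires OnAbelDeath.
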(event Custom|GiveQuest
  (Default|GiveQuest (Variables|Default|GetAC_Quest) "/Game/System/Quests/_Debug/DA_Quest_CainToAbel.DA_Quest_CainToAbel"))

(event Custom|CompleteQuest
  (Default|UpdateQuestStage (Variables|Default|GetAC_Quest) "/Game/System/Quests/_Debug/DA_Quest_CainToAbel.DA_Quest_CainToAbel" 3 true)
  (Default|CallOnAbelDeath))

(event EventInteract
  (params (PlayerCharacter :type Player%20Object%20Reference))
  (bind _ac_dialogue (Variables|Default|GetAC_Dialogue))
  (bind _ac_dialogue_2 (Variables|Default|GetAC_Dialogue))
  (switch int (Default|GetQuestStageIndex (Variables|Default|GetAC_Quest) "/Game/System/Quests/_Debug/DA_Quest_CainToAbel.DA_Quest_CainToAbel") ; Check quest stage (-1 if quest was not given)
    (:0
      (Default|StartDialogue _ac_dialogue "/Game/System/Dialogues/_Debug/DA_Dialogue_Cain_01.DA_Dialogue_Cain_01")
      (EventDispatchers|AssignOnQuestIndex _ac_dialogue (delegate Custom|GiveQuest)))
    (:2
      (Default|StartDialogue _ac_dialogue_2 "/Game/System/Dialogues/_Debug/DA_Dialogue_Cain_02.DA_Dialogue_Cain_02")
      (EventDispatchers|AssignOnQuestIndex _ac_dialogue_2 (delegate Custom|CompleteQuest)))))

(fn ConstructionScript
  (|CallParentFunction))