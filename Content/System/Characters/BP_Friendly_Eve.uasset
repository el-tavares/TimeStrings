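; BP_Friendly_Eve is the friendly NPC Eve, who advances the Adan-to-Eve quest through dialogue.
; On interaction it checks that quest's stage through the quest component and, at stage 1 only, starts Eve's dialogue.
; It then binds UpdateQuest to the dialogue component's quest-index event, which moves the quest to stage 2 without completing it.
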(event Custom|UpdateQuest
  (Default|UpdateQuestStage (Variables|Default|GetAC_Quest) "/Game/System/Quests/_Debug/DA_Quest_AdanToEve.DA_Quest_AdanToEve" 2 false))

(event EventInteract
  (params (Instigator :type Actor%20Object%20Reference))
  (bind _ac_dialogue (Variables|Default|GetAC_Dialogue))
  (switch int (Default|GetQuestStageIndex (Variables|Default|GetAC_Quest) "/Game/System/Quests/_Debug/DA_Quest_AdanToEve.DA_Quest_AdanToEve")
    (:1
      (Default|StartDialogue _ac_dialogue "/Game/System/Dialogues/_Debug/DA_Dialogue_Eve_01.DA_Dialogue_Eve_01")
      (EventDispatchers|BindEventtoOnQuestIndex _ac_dialogue (delegate Custom|UpdateQuest)))))

(fn ConstructionScript
  (|CallParentFunction))