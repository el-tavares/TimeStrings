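; BP_NPC_QuestGiver is an NPC that offers a quest to the player through dialogue.
; On Interact it checks the stage of DataQuest in the quest component, and only stage zero (quest not given) starts DataDialogue.
; It then binds GiveQuest to the dialogue's quest-index event, so that event grants DataQuest through the quest component.
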(event Custom|GiveQuest
  (Default|GiveQuest (Variables|Default|GetAC_Quest) (Variables|Default|GetDataQuest)))

(event EventInteract
  (params (Instigator :type Actor%20Object%20Reference))
  (bind _ac_dialogue (Variables|Default|GetAC_Dialogue))
  (switch int (Default|GetQuestStageIndex (Variables|Default|GetAC_Quest) (Variables|Default|GetDataQuest)) ; Check quest stage (0 if quest was not given)
    (:0
      (Default|StartDialogue _ac_dialogue (Variables|Default|GetDataDialogue))
      (EventDispatchers|AssignOnQuestIndex _ac_dialogue (delegate Custom|GiveQuest)))))

(fn ConstructionScript
  (|CallParentFunction))