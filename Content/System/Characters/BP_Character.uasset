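; Base character Blueprint handling health, shield, movement and weapon combat, with hit and team hooks for children and other systems.
; Digital damage drains the shield, health takes damage only once it is empty, and death triggers ragdoll.
; AddWeapon destroys the held weapon, then spawns a sword-shield or rifle, or unarms on a repeat selection.
; Attack, timed damage-reducing defense, shoot and reload calls forward to that weapon, alongside walk toggle and montage-gated dash.
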(event Custom|OnHit
  ;[0 0 0] On damage
)

(event Custom|LightAttack
  (params (StartingSection :type Name) (PlayRate :type Float%20%28double-precision%29) (BaseDamage :type Float%20%28single-precision%29))
  ;[0 0 0] Attacks
  (bind _meleeweapon (Variables|Default|GetMeleeWeapon)
    (:then
      (if (not (Variables|Default|GetbAttacking))
        (Default|LightAttack _meleeweapon PlayRate StartingSection BaseDamage)
        (Variables|Default|SetbAttacking true)
        (EventDispatchers|BindEventtoOnAttackEnd _meleeweapon (delegate Custom|OnAttackEnd)) ; Called by melee at notify montage
      ))
    (:else)))

(event Custom|OnDeath
  (bind _mesh (Variables|Character|GetMesh))
  ;[0 0 0] On death
  (Physics|SetSimulatePhysics _mesh true)
  (Collision|SetCollisionEnabled _mesh "PhysicsOnly")
  (Collision|SetCollisionEnabled (Variables|Collision|GetCapsuleComponent) "NoCollision")
  (Variables|Default|SetbDead true))

(event Custom|OnAttackEnd
  ;[0 0 0] Attacks
  (Variables|Default|SetbAttacking false))

(event Custom|AddWeapon
  (params (NewWeapon :type E_Weapon%20Enum :default "NewEnumerator3") (WeaponType :type E_WeaponType%20Enum :default "NewEnumerator0"))
  (bind _mesh (Variables|Character|GetMesh))
  ;[0 0 0] Add weapon
  (bind _meleeweapon (Variables|Default|GetMeleeWeapon) ; Start destroying every weapon
    (:then
      (Actor|DestroyActor _meleeweapon))
    (:else
      (bind _rangedweapon (Variables|Default|GetRangedWeapon)
        (:then
          (Actor|DestroyActor _rangedweapon))
        (:else
          _))))
  (if (Utilities|Enum|Equal(Enum) WeaponType (Variables|Default|GetCurrentWeaponType))
    (Components|SkeletalMesh|AnimationBlueprintLinking|LinkAnimClassLayers (Variables|Character|GetMesh) "/Game/System/Animations/ABP_Unarmed.ABP_Unarmed_C") ; Set unarmed if input has same weapon as before
    (Variables|Default|SetCurrentWeaponType "NewEnumerator0")
    (else
      (bind _returnvalue (Game|SpawnActorfromClass (Utilities|Select :Index NewWeapon :NewEnumerator3 0 :NewEnumerator0 "/Game/System/Weapons/BP_SwordShield.BP_SwordShield_C" :NewEnumerator1 "/Game/System/Weapons/BP_Rifle.BP_Rifle_C") (Transformation|GetActorTransform) "Undefined" "MultiplyWithRoot" self 0)) ; If diferent input, spawn a weapon
      (bind _meleeweapon_2 (Class|BPIWeapon|GetWeaponMelee(Message) _returnvalue))
      (Utilities|IsValid _meleeweapon_2 ; Validate if is a melee weapon
        (:Is%20Valid
          (bind _output_get (Variables|Default|SetMeleeWeapon _meleeweapon_2))
          (Variables|Default|SetCurrentWeaponType "NewEnumerator1")
          (Default|AttachtoSkeletal _output_get _mesh))
        (:Is%20Not%20Valid
          (bind _rangedweapon_2 (Class|BPIWeapon|GetWeaponRanged(Message) _returnvalue)) ; Is ranged weapon if is not a melee
          (Variables|Default|SetCurrentWeaponType "NewEnumerator2")
          (bind _output_get_2 (Variables|Default|SetRangedWeapon _rangedweapon_2))
          (Default|AttachtoSkeletal _output_get_2 _mesh)
          (Utilities|FlowControl|DoOnce false ; Reaload at first time getting the ranged weapon
            (:Completed
              (CallFunction|Reload 1.0))))))))

(event Custom|Dash
  ;[0 0 0] Dash
  (Utilities|FlowControl|Gate false :!label _label ; Close when start montage and open when it's blending out
    (:Exit
      (Animation|Montage|PlayMontage (Variables|Character|GetMesh) "/Game/Art/Animations/Unarmed/M_Unrmd_Dash_Montage.M_Unrmd_Dash_Montage"
        (:then
          (goto _label Close))
        (:OnBlendOut
          (goto _label Open))))))

(event Custom|Walk
  (bind _charactermovement (Variables|Character|GetCharacterMovement))
  ;[0 0 0] Walk
  (Utilities|FlowControl|FlipFlop
    (:A
      (Variables|/Script/Engine.CharacterMovementComponent|SetMaxWalkSpeed _charactermovement 2e+02))
    (:B
      (Variables|/Script/Engine.CharacterMovementComponent|SetMaxWalkSpeed _charactermovement 6e+02))))

(event Custom|StartDefending
  ;[0 0 0] Defend
  (bind _meleeweapon (Variables|Default|GetMeleeWeapon)
    (:then
      (Variables|Default|SetbDefending true)
      (Default|StartDefending _meleeweapon)
      (Variables|Default|SetDefendMultiply 0.5)
      (Utilities|FlowControl|Delay 4.0)
      (Development|PrintString "Defense ended")
      (Variables|Default|SetDefendMultiply 1.0)
      (Utilities|FlowControl|Delay 2.0)
      (Development|PrintString "Defense ability ready")
      (Variables|Default|SetbDefending false))
    (:else)))

(event Custom|StartShooting
  (params (PlayRate :type Float%20%28single-precision%29) (BaseDamage :type Float%20%28single-precision%29))
  ;[0 0 0] Shoot
  (bind _rangedweapon (Variables|Default|GetRangedWeapon)
    (:then
      (Default|StartShooting _rangedweapon PlayRate BaseDamage)
      (Variables|Default|SetbShooting true))
    (:else)))

(event Custom|StopShooting
  ;[0 0 0] Shoot
  (bind _rangedweapon (Variables|Default|GetRangedWeapon)
    (:then
      (Default|StopShooting _rangedweapon)
      (Variables|Default|SetbShooting false))
    (:else)))

(event Custom|Reload
  (params (PlayRate :type Float%20%28double-precision%29))
  ;[0 0 0] Reload
  (bind _rangedweapon (Variables|Default|GetRangedWeapon)
    (:then
      (Default|Reload _rangedweapon PlayRate))
    (:else)))

(event Custom|HeavyAttack
  (params (PlayRate :type Float%20%28double-precision%29) (BaseDamage :type Float%20%28single-precision%29))
  ;[0 0 0] Attacks
  (bind _meleeweapon (Variables|Default|GetMeleeWeapon)
    (:then
      (if (not (Variables|Default|GetbAttacking))
        (Default|HeavyAttack _meleeweapon PlayRate BaseDamage)
        (Variables|Default|SetbAttacking true)
        (EventDispatchers|BindEventtoOnAttackEnd (stale Custom|LightAttack _meleeweapon) (delegate Custom|OnAttackEnd)) ; Called by melee at notify montage
      ))
    (:else)))

(event Game|Damage|EventAnyDamage
  (params (Damage :type Float%20%28single-precision%29) (DamageType :type Damage%20Type%20Object%20Reference) (InstigatedBy :type Controller%20Object%20Reference) (DamageCauser :type Actor%20Object%20Reference))
  ;[0 0 0] On damage
  (if (and (== (Utilities|GetClass DamageType) "/Game/System/Weapons/DT_Digital.DT_Digital_C") (> (Variables|Default|GetCurrentShield) 0.0)) ; Check if is digital and has shield
    (Variables|Default|SetCurrentShield (Math|Float|Clamp(Float) (- (Variables|Default|GetCurrentShield) (* Damage (Variables|Default|GetDefendMultiply))) 0.0 (Variables|Default|GetMaxShield)))
    (elif (not (> (Variables|Default|GetCurrentShield) 0.0))
      (bind _output_get (Variables|Default|SetCurrentHealth (Math|Float|Clamp(Float) (- (Variables|Default|GetCurrentHealth) (* Damage (Variables|Default|GetDefendMultiply))) 0.0 (Variables|Default|GetMaxHealth))))
      (if (<= _output_get 0.0)
        (CallFunction|OnDeath)
        (else
          (CallFunction|OnHit))))))

(fn ConstructionScript
  (Variables|Default|SetCurrentHealth (Variables|Default|GetMaxHealth))
  (Variables|Default|SetCurrentShield (Variables|Default|GetMaxShield)))

(fn GetCharacter
  (return self))

(fn GetCharacterMovementComponent
  (return (Variables|Character|GetCharacterMovement)))

(fn GetTeamIndex
  (return (Variables|Default|GetTeamIndex)) ; 0 for neutrals, 1 for enemies
)