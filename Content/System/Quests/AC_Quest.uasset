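; Quest actor component that gives, advances and resets quests, delegating stage state to the QuestData passed into each call.
; GiveQuest uses a DoOnce to fire only once per component, sending the quest message to the player character and setting stage 1.
; UpdateQuestStage and ResetQuest forward to QuestData with debug prints; resetting leaves the DoOnce closed.
; GetQuestStageIndex returns the quest's current stage.
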(event Custom|GiveQuest
  (params (QuestData :type PDA%20Quest%20Object%20Reference))
  ;[0 0 0] Give quest
  (Utilities|FlowControl|DoOnce false
    (:Completed
      (Class|BPIPlayer|ReceiveQuest(Message) (Game|GetPlayerCharacter 0) QuestData)
      (Development|PrintString "Quest given" true true "(R=1.000000,G=1.000000,B=1.000000,A=1.000000)" 1.0)
      (CallFunction|UpdateQuestStage QuestData 1 false))))

(event Custom|UpdateQuestStage
  (params (QuestData :type PDA%20Quest%20Object%20Reference) (StageIndex :type Integer) (IsCompleted :type Boolean))
  ;[0 0 0] Update quest stage
  (Default|UpdateStage QuestData StageIndex IsCompleted)
  (Development|PrintString "Quest updated" true true "(R=1.000000,G=1.000000,B=1.000000,A=1.000000)" 1.0)
  (Development|PrintString "Quest completed" IsCompleted true "(R=1.000000,G=1.000000,B=1.000000,A=1.000000)" 1.0))

(event Custom|ResetQuest
  (params (QuestData :type PDA%20Quest%20Object%20Reference))
  ;[0 0 0] Reset quest
  (Default|ResetQuest QuestData)
  (Development|PrintString "Quest reseted" true true "(R=1.000000,G=1.000000,B=1.000000,A=1.000000)" 1.0))

(fn GetQuestStageIndex
  (params (QuestData :type PDA%20Quest%20Object%20Reference))
  (return (Variables|/Game/System/Quests/PDA_Quest.PDA_Quest_C|GetStageIndex QuestData)))