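; AC_Dialogue is a component that runs dialogue from a data asset, showing the WBP_Dialogue widget and disabling player pawn input until the conversation ends.
; GetDialogueData returns the speaker, line and options for a given index, splitting each options entry on "::".
; It also calls the quest-index notification on the step after QuestIndex and ends the dialogue once the index runs past the last line.
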(event Custom|StartDialogue
  (params (DataDialogue :type PDA%20Dialogue%20Object%20Reference))
  (Variables|Default|SetDataDialogue DataDialogue)
  (bind _returnvalue (UserInterface|CreateWidget "/Game/System/Widgets/WBP_Dialogue.WBP_Dialogue_C" 0 self))
  (UserInterface|Viewport|AddtoViewport _returnvalue 0)
  (Input|DisableInput (Game|Player|GetPlayerPawn 0) (Game|GetPlayerController 0)))

(event Custom|EndDialogue
  (Widget|RemovefromParent (stale Custom|StartDialogue _returnvalue))
  (Input|EnableInput (Game|Player|GetPlayerPawn 0) 0))

(fn GetDialogueData
  (params (DialogueIndex :type Integer))
  (bind _datadialogue (Variables|Default|GetDataDialogue)
    (:then
      (for (_array_element _array_index) (Variables|/Game/System/Dialogues/PDA_Dialogue.PDA_Dialogue_C|GetDialogue _datadialogue) ; For each dialogue from data asset...
        (if (== DialogueIndex _array_index) ; Check if dialogue index matches array's index
          (if (== DialogueIndex (+ (Variables|/Game/System/Dialogues/PDA_Dialogue.PDA_Dialogue_C|GetQuestIndex (Variables|Default|GetDataDialogue)) 1)) ; Check if index before was a quest
            (Default|CallOnQuestIndex))
          (for (_array_element_2 _array_index_2) (Variables|/Game/System/Dialogues/PDA_Dialogue.PDA_Dialogue_C|GetOptions (Variables|Default|GetDataDialogue)) ; For each options from data asset..
            (if (== DialogueIndex _array_index_2) ; Check if option index matches array's index
              (return (Variables|/Game/System/Dialogues/PDA_Dialogue.PDA_Dialogue_C|GetSpeaker (Variables|Default|GetDataDialogue)) _array_element (Utilities|String|ParseIntoArray (Utilities|String|ToString(Text) _array_element_2) "::"))))
          (elif (== DialogueIndex (Utilities|Array|Length (Variables|/Game/System/Dialogues/PDA_Dialogue.PDA_Dialogue_C|GetDialogue _datadialogue))) ; Check if is the last dialogue
            (CallFunction|EndDialogue)))))
    (:else
      (Development|PrintString "No Data Dialogue was applied" true true "(R=1.000000,G=1.000000,B=1.000000,A=1.000000)"))))