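; Ranged weapon Blueprint that fires projectiles and reloads from the owning character's ammo reserve.
; A looping shoot montage drives firing through notifies: one spawns a projectile and spends ammo, another stops shooting when the magazine empties.
; Reload moves clamped ammo from the reserve as its montage starts, and both actions mirror the weapon's count onto the character.
; Line and multi-sphere trace helpers probe for pawns ahead of the owner.
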(event Custom|StartShooting
  (params (PlayRate :type Float%20%28single-precision%29) (BaseDamage :type Float%20%28single-precision%29))
  (bind _ownercharacter (Variables|Default|GetOwnerCharacter))
  ;[0 0 0] Shoot
  (if (> (Variables|Ranged|GetCurrentAmmo) 0) ; Check if weapon has ammo
    (bind _notifyname (Animation|Montage|PlayMontage (Variables|/Script/Engine.Character|GetMesh (Variables|Default|GetOwnerCharacter)) (Variables|Ranged|GetShootMontage) PlayRate) ; This montage is looping, so only stops by notify (IT IGNORES INPUT)
      (:OnNotifyBegin
        (switch name _notifyname
          (:Shoot
            (Game|SpawnActorfromClass "/Game/System/Weapons/Projectile.Projectile_C" (Transformation|GetWorldTransform (Variables|Default|GetArrow)) "Undefined" "MultiplyWithRoot" _ownercharacter BaseDamage (Transformation|GetActorLocation _ownercharacter) 0)
            (bind _result (Math|Integer|DecrementInt (Variables|Ranged|GetCurrentAmmo))
              (:%20%20
                (bind _output_get (Variables|Ranged|SetCurrentAmmo _result))
                (Variables|/Game/System/Characters/BP_Character.BP_Character_C|SetWeaponAmmo (Variables|Default|GetOwnerCharacter) _output_get) ; Save weapon ammo on character
              )))
          (:CheckAmmo
            (if (not (> (Variables|Ranged|GetCurrentAmmo) 0)) ; Check ammo every shoot
              (Default|CallOnAnimationEnd)
              (CallFunction|StopShooting))))))))

(event Custom|Reload
  (params (PlayRate :type Float%20%28single-precision%29))
  (bind _ownercharacter (Variables|Default|GetOwnerCharacter))
  ;[0 0 0] Reload
  (if (not (>= (Variables|Ranged|GetCurrentAmmo) (Variables|Ranged|GetMaxAmmo))) ; Check if need ammo
    (if (> (Variables|/Game/System/Characters/BP_Character.BP_Character_C|GetCharAmmo _ownercharacter) 0) ; Check if character has ammo
      (Animation|Montage|PlayMontage (Variables|/Script/Engine.Character|GetMesh _ownercharacter) (Variables|Ranged|GetReloadMontage) PlayRate
        (:then
          (bind _output_get (Variables|Ranged|SetAmmoToAdd (Math|Integer|Clamp(Integer) (- (Variables|Ranged|GetMaxAmmo) (Variables|Ranged|GetCurrentAmmo)) 0 (Variables|/Game/System/Characters/BP_Character.BP_Character_C|GetCharAmmo (Variables|Default|GetOwnerCharacter)))))
          (bind _output_get_2 (Variables|/Game/System/Characters/BP_Character.BP_Character_C|SetCharAmmo (Variables|Default|GetOwnerCharacter) (- (Variables|/Game/System/Characters/BP_Character.BP_Character_C|GetCharAmmo (Variables|Default|GetOwnerCharacter)) _output_get))) ; Update character's ammo
          (bind _output_get_3 (Variables|Ranged|SetCurrentAmmo (+ (Variables|Ranged|GetCurrentAmmo) _output_get))) ; Add the necessary ammo to \ncurrent weapon's ammo
          (Variables|/Game/System/Characters/BP_Character.BP_Character_C|SetWeaponAmmo (Variables|Default|GetOwnerCharacter) _output_get_3) ; Save weapon ammo on character
        )
        (:OnCompleted
          (Default|CallOnAnimationEnd) ; Will be called completes animation
        )))))

(event Custom|StopShooting
  ;[0 0 0] Shoot
  (Animation|Montage|MontageStop (Components|SkeletalMesh|GetAnimInstance (Variables|/Script/Engine.Character|GetMesh (Variables|Default|GetOwnerCharacter))) 0.2 (Variables|Ranged|GetShootMontage)))

(fn ConstructionScript
  (|CallParentFunction))

(fn GetWeaponRanged
  (return self))