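; Base weapon Blueprint that attaches to a character and deals team-filtered damage.
; AttachToSkeletal snaps the Primary and optional Secondary components to sockets, caches the owning character and links the weapon's anim class layers to its mesh.
; DamageAllNonTeam applies physical damage to hit actors on other teams, skipping those in ActorsBeenDamaged, and reports each as an AI damage event.
; GetWeaponMelee and GetWeaponRanged are empty stubs.
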(event Custom|AttachToSkeletal
  (params (Skeletal%20Mesh :type Skeletal%20Mesh%20Component%20Object%20Reference))
  (bind _secondary (Variables|Default|GetSecondary))
  ;[0 0 0] At attachment
  (Utilities|IsValid Skeletal%20Mesh
    (:Is%20Valid
      (Utilities|FlowControl|Sequence
        (:then_0
          (Transformation|AttachComponentToComponent (Variables|Default|GetPrimary) Skeletal%20Mesh (Variables|Weapon|GetPrimarySocketName) "SnapToTarget" "SnapToTarget" "SnapToTarget" true)
          (Utilities|IsValid _secondary
            (:Is%20Valid
              (Transformation|AttachComponentToComponent _secondary Skeletal%20Mesh (Variables|Weapon|GetSecondarySocketName) "SnapToTarget" "SnapToTarget" "SnapToTarget" true))))
        (:then_1
          (bind _returnvalue (Class|BPICharacter|GetCharacter(Message) (Components|GetOwner Skeletal%20Mesh)))
          (bind _output_get (Variables|Weapon|SetOwnerCharacter _returnvalue)) ; After attach, saves character's data
          (Components|SkeletalMesh|AnimationBlueprintLinking|LinkAnimClassLayers (Variables|/Script/Engine.Character|GetMesh _output_get) (Variables|Weapon|GetAnimClassToLink)) ; Update type of animation
        )))))

(fn ConstructionScript)

(fn DamageAllNonTeam
  (params (HitResults :type Array%20of%20Hit%20Result%20Structures) (BaseDamage :type Float%20%28single-precision%29))
  (bind _ownercharacter (Variables|Weapon|GetOwnerCharacter))
  (for _array_element HitResults
    (bind _index (Class|BPICharacter|GetTeamIndex(Message) (.HitActor (Collision|BreakHitResult _array_element)))) ; Check if hitted actor is same team and was not already damaged
    (if (and (!= _index (Variables|/Game/System/Characters/BP_Character.BP_Character_C|GetTeamIndex _ownercharacter)) (not (Utilities|Array|ContainsItem (LocalVariables|GetActorsBeenDamaged) (.HitActor (Collision|BreakHitResult _array_element)))))
      (Game|Damage|ApplyDamage (.HitActor (Collision|BreakHitResult _array_element)) BaseDamage 0 _ownercharacter "/Game/System/Weapons/DT_Physical.DT_Physical_C")
      (Class|AISenseDamage|ReportDamageEvent (.HitActor (Collision|BreakHitResult _array_element)) _ownercharacter BaseDamage (Transformation|GetActorLocation _ownercharacter) "0, 0, 0" "None")
      (Utilities|Array|AddUnique (LocalVariables|GetActorsBeenDamaged) (.HitActor (Collision|BreakHitResult _array_element)))))
  (return))

(fn GetWeaponMelee
  (return 0))

(fn GetWeaponRanged
  (return 0))