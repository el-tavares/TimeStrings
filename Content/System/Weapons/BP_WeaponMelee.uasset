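; Melee weapon Blueprint that plays light attack, heavy attack and defense montages on its owner character.
; Montage notifies drive attacks: On Hit sphere-traces for Pawns ahead of the owner and passes hits to DamageAllNonTeam, while Can Attack signals attack end.
; Light attacks select a montage section, and heavy attacks trace farther.
; Defending plays a looping montage that is stopped after a short fixed delay.
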(event Custom|LightAttack
  (params (PlayRate :type Float%20%28single-precision%29) (StartingSection :type Name :default "Attack_1") (BaseDamage :type Float%20%28single-precision%29))
  ;[0 0 0] Attacks
  (bind _notifyname (Animation|Montage|PlayMontage (Variables|/Script/Engine.Character|GetMesh (Variables|Default|GetOwnerCharacter)) (Variables|Melee|GetLightAttackMontage) PlayRate 0.0 StartingSection) ; Light attack montages has specific sections
    (:OnNotifyBegin
      (switch name _notifyname
        (:OnHit
          (bind _outhits (Utilities|MultiSphereTrace 7e+01 1.5e+02))
          (CallFunction|DamageAllNonTeam _outhits BaseDamage))
        (:CanAttack
          (Default|CallOnAttackEnd))))))

(event Custom|HeavyAttack
  (params (PlayRate :type Float%20%28single-precision%29) (BaseDamage :type Float%20%28single-precision%29))
  ;[0 0 0] Attacks
  (bind _notifyname (Animation|Montage|PlayMontage (Variables|/Script/Engine.Character|GetMesh (Variables|Default|GetOwnerCharacter)) (Variables|Melee|GetHeavyAttackMontage) PlayRate)
    (:OnNotifyBegin
      (switch name _notifyname
        (:OnHit
          (bind _outhits (Utilities|MultiSphereTrace 7e+01 1.8e+02))
          (CallFunction|DamageAllNonTeam _outhits BaseDamage))
        (:CanAttack
          (Default|CallOnAttackEnd))))))

(event Custom|StartDefending
  (bind _defensemontage (Variables|Melee|GetDefenseMontage))
  (bind _ownercharacter (Variables|Default|GetOwnerCharacter))
  (bind _mesh (Variables|/Script/Engine.Character|GetMesh _ownercharacter))
  ;[0 0 0] Defense
  (Animation|Montage|PlayMontage _mesh _defensemontage 1.3 ; Defend animation montages has looping section
    (:then
      (Utilities|FlowControl|Delay 0.4)
      (Animation|Montage|MontageStop (Components|SkeletalMesh|GetAnimInstance _mesh) 0.2 _defensemontage))))

(fn ConstructionScript
  (|CallParentFunction))

(fn GetWeaponMelee
  (return self))